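; BP_GridSpawner lays out a 19×19 grid of BP_GridMarker actors across the GameBoard on BeginPlay.
; It derives the grid's corner and spacing from the board's actor bounds, inset by a fixed margin on each side.
; PlaceMarkers loops over rows and columns, spawning each marker with its indices and a hit-box size matching the cell spacing.
; A helper converts row and column to a flat index but is not called here.
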(event `self.ReceiveBeginPlay`
  (`self.PlaceMarkers`))

(fn `FlattenGridIndices`
  (params (Row :type Integer) (Column :type Integer))
  (returns (Index :type Integer))
  (return (+ (* Row (`self.gridSize`)) Column)))

(fn `GetGridMarkerGeometries`
  (params (Row :type Integer) (Column :type Integer))
  (returns (Location :type "Vector Structure") (`Available Hit Box Vector` :type "Vector Structure"))
  (bind (_bottomleft _offsetvector) (`self.GetPlayAreaGeometries`))
  (return (+ _bottomleft (`KismetMathLibrary.MakeVector` (* Row (.x _offsetvector)) (* Column (.y _offsetvector)) 1.0)) _offsetvector))

(fn `GetPlayAreaGeometries`
  (returns (BottomLeft :type "Vector Structure") (OffsetVector :type "Vector Structure"))
  (bind (_origin _boxextent) (`self.GetActorBounds` (`self.gameBoard`) false false))
  (bind _returnvalue (`KismetMathLibrary.Conv_IntToDouble` (- (`self.gridSize`) 1)))
  (bind _returnvalue_2 (- (.x _boxextent) 100))
  (bind _returnvalue_3 (- (.y _boxextent) 100))
  (return (`KismetMathLibrary.MakeVector` (- (.x _origin) _returnvalue_2) (- (.y _origin) _returnvalue_3) (.z _origin)) (`KismetMathLibrary.MakeVector` (/ (* _returnvalue_2 2) _returnvalue) (/ (* _returnvalue_3 2) _returnvalue) 30.0)))

(fn `PlaceMarkers`
  (bind _returnvalue (- (`self.gridSize`) 1))
  (for _index (range (+ _returnvalue 1))
    (for _index_2 (range (+ _returnvalue 1))
      (bind (_location _available_hit_box_vector) (`self.GetGridMarkerGeometries` _index _index_2))
      (`|SpawnActorFromClass` "/Game/BP_GridMarker.BP_GridMarker_C" (`KismetMathLibrary.Conv_VectorToTransform` _location) "Undefined" "MultiplyWithRoot" null _index _index_2 _available_hit_box_vector null))))

(fn `UserConstructionScript`
  (set `self.gridSize` 19))