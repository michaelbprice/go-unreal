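; BP_GridMarker is a clickable grid point on a two-color stone board that stores its row and column.
; Clicking its HitBox spawns a black or white stone just above it, based on CurrentPlayer in BP_GameState, then flips CurrentPlayer to the other color.
; The construction script sizes the hit box from AvailableHitBoxSize.
; The click handler does no occupancy check before spawning.
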(event `self.HitBox.OnClicked`
  (params (TouchedComponent :type "PrimitiveComponent Object Reference") (ButtonPressed :type "Key Structure"))
  (bind _asbp_game_state (cast `/Game/BP_GameState` (`GameplayStatics.GetGameState`)))
  (bind _origin (`self.GetStoneGeometries`))
  (switch `/Game/EPlayerColor` (`/Game/BP_GameState.currentPlayer` _asbp_game_state)
    (:`NewEnumerator0`
      (bind _returnvalue (`KismetMathLibrary.Conv_VectorToTransform` _origin))
      (`|SpawnActorFromClass` "/Game/BP_Stone_Black.BP_Stone_Black_C" _returnvalue "Undefined" "MultiplyWithRoot" null null))
    (:`NewEnumerator1`
      (`|SpawnActorFromClass` "/Game/BP_Stone_White.BP_Stone_White_C" _returnvalue "Undefined" "MultiplyWithRoot" null null)))
  (`self.FlipStoneColor`))

(fn `FlipStoneColor`
  (bind _asbp_game_state (cast `/Game/BP_GameState` (`GameplayStatics.GetGameState`)))
  (switch `/Game/EPlayerColor` (`/Game/BP_GameState.currentPlayer` _asbp_game_state)
    (:`NewEnumerator0`
      (set `/Game/BP_GameState.currentPlayer` "NewEnumerator1" _asbp_game_state))
    (:`NewEnumerator1`
      (set `/Game/BP_GameState.currentPlayer` "NewEnumerator0" _asbp_game_state))))

(fn `GetGridIndices`
  (returns (Row :type Integer) (Column :type Integer))
  (return (`self.row`) (`self.column`)))

(fn `GetStoneGeometries`
  (returns (Origin :type "Vector Structure"))
  (return (`KismetMathLibrary.MakeVector` (.x (`self.K2_GetActorLocation`)) (.y (`self.K2_GetActorLocation`)) (+ (.z (`self.K2_GetActorLocation`)) 35.0))))

(fn `UserConstructionScript`
  (`BoxComponent.SetBoxExtent` (`self.HitBox`) (* (`self.availableHitBoxSize`) (0.5 0.5 0.66)) true))